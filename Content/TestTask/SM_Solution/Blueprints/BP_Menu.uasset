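; In-world menu actor that switches between Main Menu, Tutorial and Settings tabs.
; On BeginPlay it spawns button actors from class arrays, stacking main buttons vertically and laying settings buttons in a row, plus a BP_Xylophone shown with Settings.
; ChangeTab toggles those actors and the tutorial widget component, including its collision.
; A visibility binding on the tutorial widget restores the main menu when that widget becomes hidden.
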(event Custom|OnTutorialVisibilityChanged
  (params (InVisibility :type ESlateVisibility%20Enum :default "Visible"))
  ;[1 0.4219 0.4219] !
  (if (Utilities|Enum|Equal(Enum) InVisibility "Hidden")
    (CallFunction|ShowMainMenu)
    (CallFunction|HideSettingsMenu)
    (CallFunction|HideTutorialMenu)))

(event EventBeginPlay
  (CallFunction|InitializeMenu))

(event Collision|EventActorBeginOverlap
  (params (OtherActor :type Actor%20Object%20Reference)))

(event EventTick
  (params (DeltaSeconds :type Float%20%28single-precision%29)))

(event EventChangeTab
  (params (Tab%20Name :type Name :default "None"))
  (switch name Tab%20Name
    (:MainMenu
      (CallFunction|ShowMainMenu)
      (CallFunction|HideSettingsMenu)
      (CallFunction|HideTutorialMenu))
    (:Tutorial
      (CallFunction|HideMainMenu)
      (CallFunction|ShowTutorialMenu))
    (:Settings
      (CallFunction|HideMainMenu)
      (CallFunction|ShowSettingsMenu))))

(fn ConstructionScript)

(fn SpawnMenuButtons
  (for (_array_element _array_index) (Variables|MainMenu|GetMenuButtonsToSpawn)
    (bind _returnvalue (Game|SpawnActorfromClass _array_element (Math|Transform|MakeTransform (+ (Transformation|GetActorLocation) (Math|Vector|MakeVector 0.0 0.0 (* _array_index (Variables|MainMenu|GetMenuButtonsOffcet)))) "0, 0, 0" "1.000000,1.000000,1.000000") "Undefined" "MultiplyWithRoot" self 0))
    (Utilities|Array|Add (Variables|MainMenu|GetMenuButtons) _returnvalue)))

(fn HideMainMenu
  (for _array_element (Variables|MainMenu|GetMenuButtons)
    (Default|HideButton _array_element)))

(fn ShowMainMenu
  (for _array_element (Variables|MainMenu|GetMenuButtons)
    (Default|ShowButton _array_element)))

(fn SpawnSettingsButtons
  (for (_array_element _array_index) (Variables|MainMenu|GetSettingsButtonsToSpawn)
    (bind _returnvalue (Game|SpawnActorfromClass _array_element (Math|Transform|MakeTransform (+ (Transformation|GetActorLocation) (Math|Vector|MakeVector 0.0 (* -6e+01 _array_index) 8e+01) "0.000000,60.000000,0.000000") "0, 0, 0" "1.000000,1.000000,1.000000") "Undefined" "MultiplyWithRoot" self 0))
    (Default|HideButton _returnvalue)
    (Utilities|Array|Add (Variables|Default|GetSettingsButtons) _returnvalue))
  (bind _returnvalue_2 (Game|SpawnActorfromClass "/Game/TestTask/SM_Solution/Blueprints/Buttons/BP_Xylophone.BP_Xylophone_C" (Math|Transform|MakeTransform (Transformation|GetActorLocation) "0, 0, 0" "1.000000,1.000000,1.000000") "Undefined" "MultiplyWithRoot" 0 0))
  (bind _output_get (Variables|Default|SetXylophone _returnvalue_2))
  (Default|Hide _output_get))

(fn InitializeMenu
  (CallFunction|SpawnMenuButtons)
  (CallFunction|SpawnSettingsButtons)
  (CallFunction|HideTutorialMenu)
  (EventDispatchers|BindEventtoOnVisibilityChanged (UserInterface|GetWidget (Variables|Default|GetWidget)) (EventDispatchers|CreateEvent :!event Custom|OnTutorialVisibilityChanged)))

(fn ShowSettingsMenu
  (for _array_element (Variables|Default|GetSettingsButtons)
    (Default|ShowButton _array_element))
  (Default|Show (Variables|Default|GetXylophone)))

(fn HideSettingsMenu
  (for _array_element (Variables|Default|GetSettingsButtons)
    (Default|HideButton _array_element))
  (Default|Hide (Variables|Default|GetXylophone)))

(fn ShowTutorialMenu
  (bind _widget (Variables|Default|GetWidget))
  (Rendering|SetVisibility _widget true false)
  (Widget|SetVisibility (UserInterface|GetWidget _widget) "Visible")
  (Collision|SetCollisionEnabled _widget "QueryOnly"))

(fn HideTutorialMenu
  (bind _widget (Variables|Default|GetWidget))
  (Rendering|SetVisibility _widget false false)
  (Widget|SetVisibility (UserInterface|GetWidget _widget) "Hidden")
  (Collision|SetCollisionEnabled _widget "NoCollision"))
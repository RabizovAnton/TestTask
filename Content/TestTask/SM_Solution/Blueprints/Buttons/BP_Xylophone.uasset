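; BP_Xylophone is an interactable, multi-section button actor that lights up like a level bar, with no sound logic in this graph.
; BeginPlay caches the root's child static meshes and their default materials in parallel arrays.
; Interact restores original materials up to and including the chosen section and sets later ones to M_ButtonBase.
; Show and Hide toggle visibility and section collision together; CanInteract always returns true.
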(event Custom|Hide
  (Rendering|SetVisibility (Variables|Default|GetDefaultSceneRoot) false true)
  (for _array_element (Variables|Default|GetSectionsArray)
    (Collision|SetCollisionEnabled _array_element "NoCollision")))

(event Custom|Show
  (Rendering|SetVisibility (Variables|Default|GetDefaultSceneRoot) true true)
  (for _array_element (Variables|Default|GetSectionsArray)
    (Collision|SetCollisionEnabled _array_element "QueryAndPhysics")))

(event EventBeginPlay
  (for _array_element (Components|GetChildrenComponents (Variables|Default|GetDefaultSceneRoot) false)
    (Utilities|Array|Add (Variables|Default|GetSectionsArray) (.AsStatic%20Mesh%20Component (Utilities|Casting|CastToStaticMeshComponent _array_element)))
    (Utilities|Array|Add (Variables|Default|GetDefaultMaterials) (Rendering|Material|GetMaterial (.AsStatic%20Mesh%20Component (Utilities|Casting|CastToStaticMeshComponent _array_element)) 0))))

(event Collision|EventActorBeginOverlap
  (params (OtherActor :type Actor%20Object%20Reference)))

(event EventTick
  (params (DeltaSeconds :type Float%20%28single-precision%29)))

(event EventInteract
  (params (InteractComponent :type Primitive%20Component%20Object%20Reference))
  (for (_array_element _array_index) (Variables|Default|GetSectionsArray)
    (Rendering|Material|SetMaterial _array_element 0 (select (<= _array_index (Utilities|Array|FindItem (Variables|Default|GetSectionsArray) InteractComponent)) (Utilities|Array|Get(acopy) (Variables|Default|GetDefaultMaterials) _array_index) "/Game/TestTask/SM_Solution/Materials/M_ButtonBase.M_ButtonBase"))))

(fn ConstructionScript)

(fn CanInteract?
  (return true))
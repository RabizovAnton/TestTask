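; BP_ButtonBase is a base Blueprint for interactable in-world buttons with a mesh and a text label.
; The construction script applies the default material and sets the label from the Name variable.
; Highlight swaps in a highlight material and reverts after a retriggerable delay, so repeated calls keep it lit.
; Show and Hide events toggle visibility and mesh collision together, while CanInteract reports the ButtonActive flag.
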(event Custom|HideButton
  (Rendering|SetVisibility (Variables|Default|GetScene) false true)
  (Collision|SetCollisionEnabled (Variables|Default|GetSM_Button) "NoCollision"))

(event Custom|ShowButton
  (Rendering|SetVisibility (Variables|Default|GetScene) true true)
  (Collision|SetCollisionEnabled (Variables|Default|GetSM_Button) "QueryAndPhysics"))

(event EventBeginPlay)

(event Collision|EventActorBeginOverlap
  (params (OtherActor :type Actor%20Object%20Reference)))

(event EventTick
  (params (DeltaSeconds :type Float%20%28single-precision%29)))

(event EventHighlight
  (bind _sm_button (Variables|Default|GetSM_Button))
  (Rendering|Material|SetMaterial _sm_button 0 (Variables|Default|GetHighlightMaterial))
  (Utilities|FlowControl|RetriggerableDelay 0.1)
  (Rendering|Material|SetMaterial _sm_button 0 (Variables|Default|GetDefaultMaterial)))

(fn ConstructionScript
  (Rendering|Material|SetMaterial (Variables|Default|GetSM_Button) 0 (Variables|Default|GetDefaultMaterial))
  (Rendering|Components|TextRender|SetText (Variables|Default|GetButtonName) (Variables|Default|GetName)))

(fn CanInteract?
  (return (Variables|Default|GetButtonActive?)))
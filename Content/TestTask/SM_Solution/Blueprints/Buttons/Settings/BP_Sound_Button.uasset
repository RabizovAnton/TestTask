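; BP_Sound_Button is an interactable sound settings button actor that switches between pressed and unpressed states.
; Each Interact event flips ButtonPressed and sets DefaultMaterial to grey when pressed or green when released.
; The Blueprint only updates this state and material variable; it contains no audio logic, and its BeginPlay, overlap and Tick events are disabled.
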(event EventBeginPlay
  (|CallParentFunction) ; This node is disabled and will not be called.\nDrag off pins to build functionality.
)

(event Collision|EventActorBeginOverlap
  (params (OtherActor :type Actor%20Object%20Reference))
  (|CallParentFunction OtherActor) ; This node is disabled and will not be called.\nDrag off pins to build functionality.
)

(event EventTick
  (params (DeltaSeconds :type Float%20%28single-precision%29))
  (|CallParentFunction DeltaSeconds) ; This node is disabled and will not be called.\nDrag off pins to build functionality.
)

(event EventInteract
  (bind _output_get (Variables|Default|SetButtonPressed? (not (Variables|Default|GetButtonPressed?))))
  (Variables|Default|SetDefaultMaterial (select _output_get "/Game/TestTask/SM_Solution/Materials/MI_Grey.MI_Grey" "/Game/TestTask/SM_Solution/Materials/MI_Green.MI_Green")))

(fn ConstructionScript
  (|CallParentFunction))